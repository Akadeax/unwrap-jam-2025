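; BP_Boat_Entrance moves a boat from a start location to an end location as an entrance sequence when play begins.
; After a configurable delay, a timeline with its play rate set from the move duration lerps the relative location of MoveScene between the two points.
; The construction script applies a uniform scale to the boat mesh.
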(event `self.ReceiveBeginPlay`
  (`SceneComponent.K2_SetRelativeLocation` (`self.MoveScene`) (`self.StartLoc`) false false)
  (`KismetSystemLibrary.Delay` (`self.DelayBeforeMoving`))
  (`TimelineComponent.SetPlayRate` (`self.TL_BoatMove`) (/ 1.0 (`self.BoatMoveDuration`)))
  (bind (_direction _movelerp) (`Timeline|TL_BoatMove` :!via `PlayFromStart`)
    (:`Update`
      (`SceneComponent.K2_SetRelativeLocation` (`self.MoveScene`) (`KismetMathLibrary.VLerp` (`self.StartLoc`) (`self.EndLoc`) _movelerp) false false))))

(fn `UserConstructionScript`
  (bind _boatscale (`self.BoatScale`))
  (`SceneComponent.SetRelativeScale3D` (`self.MS_Boat`) (`KismetMathLibrary.MakeVector` _boatscale _boatscale _boatscale)))