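; BP_FXTester is a VFX test actor that moves a scene component to preview an acceleration effect in motion.
; On BeginPlay it snaps MoveScene to the start location, waits a configurable delay, then plays a timeline scaled to the move duration.
; The timeline lerps the relative location toward the end point, and its Change Direction event restarts the FXSAcceleration effect by deactivating and reactivating it.
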(event `self.ReceiveBeginPlay`
  (bind _fxs_acceleration (`self.FXS_Acceleration`))
  (`SceneComponent.K2_SetRelativeLocation` (`self.MoveScene`) (`self.StartLoc`) false false)
  (`KismetSystemLibrary.Delay` (`self.DelayBeforeMoving`))
  (`TimelineComponent.SetPlayRate` (`self.TLObjectMove`) (/ 1.0 (`self.ObjectMoveDuration`)))
  (bind (_direction _movelerp) (`Timeline|TLObjectMove` :!via `PlayFromStart`)
    (:`Update`
      (`SceneComponent.K2_SetRelativeLocation` (`self.MoveScene`) (`KismetMathLibrary.VLerp` (`self.StartLoc`) (`self.EndLoc`) _movelerp) false false))
    (:`ChangeDirection`
      (`ActorComponent.Deactivate` _fxs_acceleration)
      (`ActorComponent.Activate` _fxs_acceleration false))))

(fn `UserConstructionScript`)