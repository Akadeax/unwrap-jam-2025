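; BP_PlatformParticles is an actor that shows a particle effect moving back and forth between two points.
; On BeginPlay it attaches the FXS_PlatformParticles system to the Traveler component.
; Each Tick advances a time value and moves Traveler along a sine-driven lerp between the Start and End component locations, giving a smooth oscillation.
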(event `self.ReceiveBeginPlay`
  (`NiagaraFunctionLibrary.SpawnSystemAttached` "/Game/VFX/FXS_PlatformParticles.FXS_PlatformParticles" (`self.Traveler`) "None" (0.0 0.0 0.0) (struct) "SnapToTargetIncludingScale"))

(event `self.ReceiveTick`
  (params (DeltaSeconds :type "Float (single-precision)"))
  (bind _output_get (set `self.Time` (+ (`self.Time`) (* DeltaSeconds 3.0))))
  (`SceneComponent.K2_SetWorldLocation` (`self.Traveler`) (`KismetMathLibrary.VLerp` (`SceneComponent.K2_GetComponentLocation` (`self.Start`)) (`SceneComponent.K2_GetComponentLocation` (`self.End`)) (/ (+ (`KismetMathLibrary.Sin` _output_get) 1.0) 2.0)) false false))

(fn `UserConstructionScript`)