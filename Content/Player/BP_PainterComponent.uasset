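; Painter component that stamps a circle material into the RT_Mask render target at a world position.
; When drawing is enabled and set to constant, it stamps at its own location every tick.
; DoDraw projects the position to screen space, maps it into a half-scale region of the canvas, then shifts it by the player camera's NDC offset.
; The final Y threshold check leaves the position unchanged.
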(event `self.ReceiveBeginPlay`
  (bind _returnvalue (`GameplayStatics.GetActorOfClass` "/Game/Player/BP_PlayerCamera.BP_PlayerCamera_C"))
  (set `self.PlayerCam` _returnvalue))

(event `self.ReceiveTick`
  (params (DeltaSeconds :type "Float (single-precision)"))
  (if (`self.DrawEnabled`)
    (if (`self.Constant`)
      (`self.DoDraw` (`self.K2_GetComponentLocation`)))))

(fn `DoDraw`
  (params (Position :type "Vector Structure"))
  (locals (CanvasPos :type "Vector2D Structure"))
  (bind (_x _y) (`KismetMathLibrary.BreakVector2D` (`local.CanvasPos`)))
  (bind (_x_2 _y_2) (`KismetMathLibrary.BreakVector2D` (`/Game/Player/BP_PlayerCamera.NDCOffset` (`self.PlayerCam`))))
  (bind (_canvas _size _context) (`KismetRenderingLibrary.BeginDrawCanvasToRenderTarget` "/Game/Global/Materials/Test/RT_Mask.RT_Mask"))
  (bind _rendertexpos (`self.WorldPosToRenderTexPos` _size Position))
  (bind _output_get (set `local.CanvasPos` (+ (- _rendertexpos (/ (`self.SizeOnTex`) (2.0 2.0))) (* _size (`KismetMathLibrary.MakeVector2D` _x_2 (+ (- 1.0 _y_2) -1.0)) (0.5 0.5)))))
  (if (> (`.Y` (`KismetMathLibrary.BreakVector2D` _output_get)) 450.0)
    (set `local.CanvasPos` (`KismetMathLibrary.MakeVector2D` _x _y)))
  (`Canvas.K2_DrawMaterial` _canvas "/Game/Global/Materials/Test/M_PaintingCircle.M_PaintingCircle" (`local.CanvasPos`) (`self.SizeOnTex`) (0.0 0.0) (1.0 1.0) 0.0 (0.5 0.5))
  (`KismetRenderingLibrary.EndDrawCanvasToRenderTarget` _context))

(fn `WorldPosToRenderTexPos`
  (params (CanvasSize :type "Vector2D Structure") (WorldPos :type "Vector Structure"))
  (returns (RenderTexPos :type "Vector2D Structure"))
  (return (* (+ (/ (`GameplayStatics.ProjectWorldToScreen` (`GameplayStatics.GetPlayerController` 0) WorldPos) (`WidgetLayoutLibrary.GetViewportSize`) (2.0 2.0)) (0.0 0.5)) CanvasSize)))