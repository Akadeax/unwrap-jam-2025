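; Player character for a side-view platformer moving along the Y axis, with running, hold-length jumps, dashing, wall slides and wall jumps.
; Tick drives dash velocity and trace-based wall sliding, then compares against previous-frame state to fire landing and slide events.
; Custom jump checks use twin ground traces, hold time and a post-dash grace window.
; Debug keys tune gravity, jump, air control, dash and wall-jump values, logged on EndPlay.
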(event Custom|DashHandler
  (params (deltaT :type Float%20%28double-precision%29))
  ;[0.15 0.15 0.15 0.5] dash
  (if (> (Variables|Dash|GetCurrentDashTime) 0.0)
    (bind _isgrounded (CallFunction|IsGrounded))
    (Variables|/Script/Engine.MovementComponent|SetVelocity (Variables|Character|GetCharacterMovement) (* (* (* (Variables|Dash|GetDashVelocity) "0.000000,1.000000,0.000000") (Variables|Default|GetDir)) (select _isgrounded 1.7 1.0)))
    (else
      (Variables|Dash|SetWasDashing false)
      (if (not (Variables|Dash|GetCanDash))
        (Variables|Dash|SetCanDash (and (AI|Components|NavMovement|IsMovingonGround (Variables|Character|GetCharacterMovement)) (<= (Variables|Dash|GetCurrentTimeBetweenDashes) 0.0)))
        (Variables|Dash|SetCurrentTimeBetweenDashes (- (Variables|Dash|GetCurrentTimeBetweenDashes) deltaT))))))

(event Custom|HandleWallSlide
  (params (DeltaTime :type Float%20%28double-precision%29))
  (bind _returnvalue (Transformation|GetActorLocation))
  (bind _returnvalue_2 (Transformation|GetActorLocation))
  (bind _returnvalue_3 (Transformation|GetActorLocation))
  (bind _charactermovement (Variables|Character|GetCharacterMovement))
  (bind _maxslidespeed (Variables|WallAbilities|GetMaxSlideSpeed))
  (bind _charactermovement_2 (Variables|Character|GetCharacterMovement))
  (bind _returnvalue_4 (Pawn|Components|CharacterMovement|GetLastUpdateVelocity _charactermovement_2))
  (bind _returnvalue_5 (Pawn|Components|CharacterMovement|GetLastUpdateVelocity _charactermovement))
  (bind _returnvalue_6 (Pawn|Components|CharacterMovement|GetLastUpdateVelocity _charactermovement_2))
  (bind _returnvalue_7 (+ _returnvalue_2 "0.000000,60.000000,0.000000"))
  (bind _returnvalue_8 (+ _returnvalue_3 "0.000000,-60.000000,0.000000"))
  (bind _returnvalue_9 (< (.z _returnvalue_5) 0.0))
  ;[0.15 0.15 0.15 0.5] wallsliding
  (bind _returnvalue_10 (Collision|LineTraceByChannel _returnvalue_2 _returnvalue_7 "TraceTypeQuery1" false 0 "None"))
  (bind _returnvalue_11 (Collision|LineTraceByChannel (- _returnvalue_2 "0.000000,0.000000,60.000000") (- _returnvalue_7 "0.000000,0.000000,60.000000") "TraceTypeQuery1" false 0 "None"))
  (bind _returnvalue_12 (Collision|LineTraceByChannel _returnvalue_3 _returnvalue_8 "TraceTypeQuery1" false 0 "None"))
  (bind _returnvalue_13 (Collision|LineTraceByChannel (- _returnvalue_3 "0.000000,0.000000,60.000000") (- _returnvalue_8 "0.000000,0.000000,60.000000") "TraceTypeQuery1" false 0 "None"))
  (if (and _returnvalue_13 _returnvalue_12)
    (Variables|WallAbilities|SetWallhangDir 1))
  (if (and _returnvalue_10 _returnvalue_11)
    (Variables|WallAbilities|SetWallhangDir -1))
  (bind _returnvalue_14 (Collision|LineTraceByChannel _returnvalue (+ _returnvalue (Math|Vector|MakeVector 0.0 0.0 (* (Components|Capsule|GetScaledCapsuleHalfHeight (Variables|Collision|GetCapsuleComponent)) -2.0))) "TraceTypeQuery1" false 0 "None"))
  (if (Math|Boolean|ANDBoolean _returnvalue_14 _returnvalue_9 (or (and _returnvalue_13 _returnvalue_12) (and _returnvalue_10 _returnvalue_11)))
    _
    (else
      _))
  (Variables|WallAbilities|SetIsSliding (and (not _returnvalue_14) (or (and _returnvalue_13 _returnvalue_12) (and _returnvalue_10 _returnvalue_11))))
  (if (and (and (not _returnvalue_14) (or (and _returnvalue_13 _returnvalue_12) (and _returnvalue_10 _returnvalue_11))) _returnvalue_9)
    (if (<= (Variables|WallAbilities|GetCurrentSlideDelay) 0.0)
      (Variables|/Script/Engine.MovementComponent|SetVelocity _charactermovement_2 (Math|Vector|MakeVector (.x _returnvalue_6) (.y _returnvalue_6) (Variables|WallAbilities|GetSlideSpeed)))
      (if (>= (Variables|WallAbilities|GetSlideSpeed) _maxslidespeed)
        (Variables|WallAbilities|SetSlideSpeed (+ (Variables|WallAbilities|GetSlideSpeed) (* (/ _maxslidespeed 2.0) DeltaTime))))
      (else
        (Variables|WallAbilities|SetCurrentSlideDelay (- (Variables|WallAbilities|GetCurrentSlideDelay) DeltaTime))
        (Variables|/Script/Engine.MovementComponent|SetVelocity _charactermovement_2 (Math|Vector|MakeVector (.x _returnvalue_4) (.y _returnvalue_4) 0.0))))
    (else
      (Variables|WallAbilities|SetCurrentSlideDelay (Variables|WallAbilities|GetMaxslideDelay))
      (Variables|WallAbilities|SetSlideSpeed 0.0))))

(event Custom|EventHandler
  (bind _currentdashtime (Variables|Dash|GetCurrentDashTime))
  ;[0.15 0.15 0.15 0.5] call anim events
  (Utilities|FlowControl|Sequence
    (:then_0
      (if (and (Variables|WallAbilities|GetIsSliding) (not (Variables|WallAbilities|GetWasSliding)))
        (Default|CallOnWallSlide)
        (elif (and (Variables|WallAbilities|GetWasSliding) (not (Variables|WallAbilities|GetIsSliding)))
          (Default|CallOnWallSlideEnd))))
    (:then_1
      (bind _isgrounded (CallFunction|IsGrounded))
      (if (and _isgrounded (not (Variables|Default|GetWasGrounded)))
        (Default|CallOnLand)))
    (:then_2
      (if (and (Variables|Dash|GetWasDashing) (not (and (> _currentdashtime 0.0) (< _currentdashtime (Variables|Dash|GetMaxDashTime)))))
        (Development|PrintString "stopped dashing")))))

(event Custom|PostTickHandler
  (bind _currentdashtime (Variables|Dash|GetCurrentDashTime))
  ;[0.15 0.15 0.15 0.5] post tick for events
  (bind _isgrounded (CallFunction|IsGrounded))
  (bind _output_get (Variables|Dash|SetIsDashing (and (> _currentdashtime 0.0) (< _currentdashtime (Variables|Dash|GetMaxDashTime)))))
  (Utilities|FlowControl|DelayUntilNextTick)
  (Variables|WallAbilities|SetWasSliding (Variables|WallAbilities|GetIsSliding))
  (Variables|Default|SetWasGrounded _isgrounded)
  (Variables|Dash|SetWasDashing _output_get))

(event Input|EnhancedActionEvents|EnhancedInputActionIA_Move
  (params (ActionValue :type Float%20%28double-precision%29) (ElapsedSeconds :type Float%20%28double-precision%29) (TriggeredSeconds :type Float%20%28double-precision%29) (InputAction :type Input%20Action%20Object%20Reference :default "/Game/Player/Input/IA_Move.IA_Move"))
  ;[0.15 0.15 0.15 0.5] base movement
  (if (and (> (Math|Float|Absolute(Float) ActionValue) 0.1) (<= (Variables|Dash|GetCurrentDashTime) 0.0))
    (Utilities|FlowControl|Sequence
      (:then_0
        (if (>= ActionValue 0.0)
          (Variables|Default|SetDir 1)
          (else
            (Variables|Default|SetDir -1))))
      (:then_1
        (Pawn|Input|AddMovementInput "0.000000,1.000000,0.000000" ActionValue false)))))

(event Input|EnhancedActionEvents|EnhancedInputActionIA_Jump
  (params (ActionValue :type Boolean) (ElapsedSeconds :type Float%20%28double-precision%29) (TriggeredSeconds :type Float%20%28double-precision%29) (InputAction :type Input%20Action%20Object%20Reference :default "/Game/Player/Input/IA_Jump.IA_Jump"))
  (bind _returnvalue (Character|CanJump))
  (bind _issliding (Variables|WallAbilities|GetIsSliding))
  (bind _walljumpvelocity (Variables|WallAbilities|GetWallJumpVelocity))
  ;[0.15 0.15 0.15 0.5] handle jumping
  (:Triggered
    (if (not _issliding)
      (Character|Jump)
      (if _returnvalue
        (Variables|Jump|SetIsPrevFrameJump true)
        (Variables|Jump|SetJumpHeldLength (+ (Utilities|Time|GetWorldDeltaSeconds) (Variables|Jump|GetJumpHeldLength)))
        (Variables|Dash|SetCanJumpPostDash false)
        (Variables|Dash|SetCurrentDashTime -0.1))))
  (:Started
    (if _issliding
      (Character|LaunchCharacter (Math|Vector|MakeVector 0.0 (* _walljumpvelocity (Variables|WallAbilities|GetWallhangDir)) (* _walljumpvelocity 1.0)) false true)
      (Default|CallOnWallJump)
      (elif _returnvalue
        (Default|CallOnJump))))
  (:Completed
    (if (not _issliding)
      (Character|StopJumping)
      (Variables|Jump|SetIsPrevFrameJump false)
      (Variables|Jump|SetJumpHeldLength 0.0)
      (Development|PrintString "end jump"))))

(event Input|EnhancedActionEvents|EnhancedInputActionIA_Dash
  (params (ActionValue :type Boolean) (ElapsedSeconds :type Float%20%28double-precision%29) (TriggeredSeconds :type Float%20%28double-precision%29) (InputAction :type Input%20Action%20Object%20Reference :default "/Game/Player/Input/IA_Dash.IA_Dash"))
  ;[0.15 0.15 0.15 0.5] dash
  (if (Variables|Dash|GetCanDash)
    (Variables|Dash|SetCurrentDashTime (Variables|Dash|GetMaxDashTime))
    (Variables|Dash|SetCanDash false)
    (Variables|Dash|SetCurrentTimeBetweenDashes (Variables|Dash|GetMaxTimeBetweenDashes))
    (Variables|Dash|SetCanJumpPostDash (Character|CanJump))
    (Default|CallOnDash)
    (Variables|Default|SetDashEnded true)))

(event Input|EnhancedActionEvents|EnhancedInputActionIA_UIStartGame
  (params (ActionValue :type Float%20%28double-precision%29) (ElapsedSeconds :type Float%20%28double-precision%29) (TriggeredSeconds :type Float%20%28double-precision%29) (InputAction :type Input%20Action%20Object%20Reference :default "/Game/Player/Input/IA_UIStartGame.IA_UIStartGame"))
  (Default|CallStartPressed))

(event EventBeginPlay
  ;[0.15 0.15 0.15 0.5] wallsliding
)

(event EventTick
  (params (DeltaSeconds :type Float%20%28single-precision%29))
  (bind _mesh (Variables|Character|GetMesh))
  ;[0.15 0.15 0.15 0.5] tick
  (Utilities|FlowControl|Sequence
    (:then_0
      (CallFunction|DashHandler DeltaSeconds)
      (CallFunction|HandleWallSlide DeltaSeconds)
      (CallFunction|EventHandler)
      (Variables|Dash|SetCurrentDashTime (- (Variables|Dash|GetCurrentDashTime) DeltaSeconds))
      (if (and (< (Variables|Dash|GetCurrentDashTime) 0.0) (Variables|Default|GetDashEnded))
        (Default|CallOnDashEnd)
        (Variables|Default|SetDashEnded false)
        (Development|PrintString "Hello"))
      (Transformation|SetWorldRotation _mesh (Math|Interpolation|RInterpTo (Transformation|GetWorldRotation _mesh) (Utilities|Select :Index (+ (Variables|Default|GetDir) 1) :Option%200 "0.000000,180.000000,0.000000" :Option%201 "0, 0, 0" :Option%202 "0, 0, 0") DeltaSeconds 1e+01) false false)
      (if (Class|KismetMathLibrary|XORBoolean (Variables|Dash|GetWasDashing) (Variables|Dash|GetIsDashing))
        (Development|PrintString "was dashing'")))
    (:then_1
      (CallFunction|PostTickHandler))))

(event EventEndPlay
  (params (EndPlayReason :type EEndPlayReason%20Enum :default "Destroyed"))
  (Utilities|FlowControl|Sequence
    (:then_0
      (Utilities|String|LogString "---------------------------------------------------------------------------------" :!label _label))
    (:then_1
      (Utilities|String|LogString (Utilities|String|Append "gravity :" (Utilities|String|ToString(Float) (Variables|/Script/Engine.CharacterMovementComponent|GetGravityScale (Variables|Character|GetCharacterMovement)))))
      (Utilities|String|LogString (Utilities|String|Append "jump vel :" (Utilities|String|ToString(Float) (Variables|/Script/Engine.CharacterMovementComponent|GetJumpZVelocity (Variables|Character|GetCharacterMovement)))))
      (Utilities|String|LogString (Utilities|String|Append "air controll :" (Utilities|String|ToString(Float) (Variables|/Script/Engine.CharacterMovementComponent|GetAirControl (Variables|Character|GetCharacterMovement)))))
      (Utilities|String|LogString (Utilities|String|Append "dash velocity :" (Utilities|String|ToString(Float) (Variables|Dash|GetDashVelocity))))
      (Utilities|String|LogString (Utilities|String|Append "walljump velocity :" (Utilities|String|ToString(Float) (Variables|WallAbilities|GetWallJumpVelocity)))))
    (:then_2
      (goto _label))))

(event Input|KeyboardEvents|DebugKeyUp
  (params (Key :type Key%20Structure :default "None") (ActionValue :type Input%20Action%20Value%20Structure))
  (bind _charactermovement (Variables|Character|GetCharacterMovement))
  ;[0.15 0.15 0.15 0.5] testing
  (:Pressed
    (Variables|/Script/Engine.CharacterMovementComponent|SetGravityScale _charactermovement (+ 0.1 (Variables|/Script/Engine.CharacterMovementComponent|GetGravityScale _charactermovement)))
    (Development|PrintString (Utilities|String|Append "gravity :" (Utilities|String|ToString(Float) (Variables|/Script/Engine.CharacterMovementComponent|GetGravityScale _charactermovement))))))

(event Input|KeyboardEvents|DebugKeyDown
  (params (Key :type Key%20Structure :default "None") (ActionValue :type Input%20Action%20Value%20Structure))
  (bind _charactermovement (Variables|Character|GetCharacterMovement))
  ;[0.15 0.15 0.15 0.5] testing
  (:Pressed
    (Variables|/Script/Engine.CharacterMovementComponent|SetGravityScale _charactermovement (- (Variables|/Script/Engine.CharacterMovementComponent|GetGravityScale _charactermovement) 0.1))
    (Development|PrintString (Utilities|String|Append "gravity :" (Utilities|String|ToString(Float) (Variables|/Script/Engine.CharacterMovementComponent|GetGravityScale _charactermovement))))))

(event Input|KeyboardEvents|DebugKeyG
  (params (Key :type Key%20Structure :default "None") (ActionValue :type Input%20Action%20Value%20Structure))
  ;[0.15 0.15 0.15 0.5] testing
  (:Pressed
    (Variables|WallAbilities|SetWallJumpVelocity (- (Variables|WallAbilities|GetWallJumpVelocity) 1e+02))
    (Development|PrintString (Utilities|String|Append "walljump velocity :" (Utilities|String|ToString(Float) (Variables|WallAbilities|GetWallJumpVelocity))))))

(event Input|KeyboardEvents|DebugKeyU
  (params (Key :type Key%20Structure :default "None") (ActionValue :type Input%20Action%20Value%20Structure))
  (bind _charactermovement (Variables|Character|GetCharacterMovement))
  ;[0.15 0.15 0.15 0.5] testing
  (:Pressed
    (Variables|/Script/Engine.CharacterMovementComponent|SetAirControl _charactermovement (+ (Variables|/Script/Engine.CharacterMovementComponent|GetAirControl _charactermovement) 0.05))
    (Development|PrintString (Utilities|String|Append "air controll :" (Utilities|String|ToString(Float) (Variables|/Script/Engine.CharacterMovementComponent|GetAirControl _charactermovement))))))

(event Input|KeyboardEvents|DebugKeyI
  (params (Key :type Key%20Structure :default "None") (ActionValue :type Input%20Action%20Value%20Structure))
  (bind _charactermovement (Variables|Character|GetCharacterMovement))
  ;[0.15 0.15 0.15 0.5] testing
  (:Pressed
    (Variables|/Script/Engine.CharacterMovementComponent|SetJumpZVelocity _charactermovement (+ (Variables|/Script/Engine.CharacterMovementComponent|GetJumpZVelocity _charactermovement) 1e+02))
    (Development|PrintString (Utilities|String|Append "jump vel :" (Utilities|String|ToString(Float) (Variables|/Script/Engine.CharacterMovementComponent|GetJumpZVelocity _charactermovement))))))

(event Input|KeyboardEvents|DebugKeyK
  (params (Key :type Key%20Structure :default "None") (ActionValue :type Input%20Action%20Value%20Structure))
  (bind _charactermovement (Variables|Character|GetCharacterMovement))
  ;[0.15 0.15 0.15 0.5] testing
  (:Pressed
    (Variables|/Script/Engine.CharacterMovementComponent|SetJumpZVelocity _charactermovement (- (Variables|/Script/Engine.CharacterMovementComponent|GetJumpZVelocity _charactermovement) 1e+02))
    (Development|PrintString (Utilities|String|Append "jump vel :" (Utilities|String|ToString(Float) (Variables|/Script/Engine.CharacterMovementComponent|GetJumpZVelocity _charactermovement))))))

(event Input|KeyboardEvents|DebugKeyJ
  (params (Key :type Key%20Structure :default "None") (ActionValue :type Input%20Action%20Value%20Structure))
  (bind _charactermovement (Variables|Character|GetCharacterMovement))
  ;[0.15 0.15 0.15 0.5] testing
  (:Pressed
    (Variables|/Script/Engine.CharacterMovementComponent|SetAirControl _charactermovement (- (Variables|/Script/Engine.CharacterMovementComponent|GetAirControl _charactermovement) 0.05))
    (Development|PrintString (Utilities|String|Append "air controll :" (Utilities|String|ToString(Float) (Variables|/Script/Engine.CharacterMovementComponent|GetAirControl _charactermovement))))))

(event Input|KeyboardEvents|DebugKeyY
  (params (Key :type Key%20Structure :default "None") (ActionValue :type Input%20Action%20Value%20Structure))
  ;[0.15 0.15 0.15 0.5] testing
  (:Pressed
    (Variables|Dash|SetDashVelocity (+ (Variables|Dash|GetDashVelocity) 1e+02))
    (Development|PrintString (Utilities|String|Append "dash velocity :" (Utilities|String|ToString(Float) (Variables|Dash|GetDashVelocity))))))

(event Input|KeyboardEvents|DebugKeyH
  (params (Key :type Key%20Structure :default "None") (ActionValue :type Input%20Action%20Value%20Structure))
  ;[0.15 0.15 0.15 0.5] testing
  (:Pressed
    (Variables|Dash|SetDashVelocity (- (Variables|Dash|GetDashVelocity) 1e+02))
    (Development|PrintString (Utilities|String|Append "dash velocity :" (Utilities|String|ToString(Float) (Variables|Dash|GetDashVelocity))))))

(event Input|KeyboardEvents|DebugKeyT
  (params (Key :type Key%20Structure :default "None") (ActionValue :type Input%20Action%20Value%20Structure))
  ;[0.15 0.15 0.15 0.5] testing
  (:Pressed
    (Variables|WallAbilities|SetWallJumpVelocity (+ (Variables|WallAbilities|GetWallJumpVelocity) 1e+02))
    (Development|PrintString (Utilities|String|Append "walljump velocity :" (Utilities|String|ToString(Float) (Variables|WallAbilities|GetWallJumpVelocity))))))

(fn ConstructionScript)

(fn CanJumpInternal
  (bind _returnvalue (Transformation|GetActorLocation))
  (bind _capsulecomponent (Variables|Collision|GetCapsuleComponent))
  (bind _returnvalue_2 (Components|Capsule|GetScaledCapsuleHalfHeight _capsulecomponent))
  (bind _returnvalue_3 (Components|Capsule|GetScaledCapsuleRadius _capsulecomponent))
  (bind _returnvalue_4 (+ _returnvalue_2 5e+01))
  (bind _returnvalue_5 (/ _returnvalue_3 2.0))
  (bind _returnvalue_6 (* _returnvalue_4 -1.0))
  (bind _returnvalue_7 (Collision|LineTraceByChannel _returnvalue (+ _returnvalue (Math|Vector|MakeVector 0.0 _returnvalue_5 _returnvalue_6)) "TraceTypeQuery1" false 0 "None" true "(R=1.000000,G=0.000000,B=0.000000,A=1.000000)" "(R=0.000000,G=1.000000,B=0.000000,A=1.000000)" 0.5))
  (bind _returnvalue_8 (Collision|LineTraceByChannel _returnvalue (+ _returnvalue (Math|Vector|MakeVector 0.0 (* _returnvalue_5 -1.0) _returnvalue_6)) "TraceTypeQuery1" false 0 "None" true "(R=1.000000,G=0.000000,B=0.000000,A=1.000000)" "(R=0.000000,G=1.000000,B=0.000000,A=1.000000)" 0.5))
  (return (and (Math|Boolean|ORBoolean (or _returnvalue_7 _returnvalue_8) (Variables|Jump|GetIsPrevFrameJump) (and (Variables|Dash|GetCanJumpPostDash) (> (Variables|Dash|GetCurrentDashTime) (* (Variables|Dash|GetJumpPostDashTime) -1.0)))) (<= (Variables|Jump|GetJumpHeldLength) (Variables|Jump|GetMaxJumpHoldTime)))))

(fn IsGrounded
  (bind _returnvalue (Transformation|GetActorLocation))
  (bind _capsulecomponent (Variables|Collision|GetCapsuleComponent))
  (bind _returnvalue_2 (Components|Capsule|GetScaledCapsuleHalfHeight _capsulecomponent))
  (bind _returnvalue_3 (Components|Capsule|GetScaledCapsuleRadius _capsulecomponent))
  (bind _returnvalue_4 (+ _returnvalue_2 5e+01))
  (bind _returnvalue_5 (/ _returnvalue_3 2.0))
  (bind _returnvalue_6 (* _returnvalue_4 -1.0))
  (bind _returnvalue_7 (Collision|LineTraceByChannel _returnvalue (+ _returnvalue (Math|Vector|MakeVector 0.0 _returnvalue_5 _returnvalue_6)) "TraceTypeQuery1" false 0 "None" true "(R=1.000000,G=0.000000,B=0.000000,A=1.000000)" "(R=0.000000,G=1.000000,B=0.000000,A=1.000000)" 0.5))
  (bind _returnvalue_8 (Collision|LineTraceByChannel _returnvalue (+ _returnvalue (Math|Vector|MakeVector 0.0 (* _returnvalue_5 -1.0) _returnvalue_6)) "TraceTypeQuery1" false 0 "None" true "(R=1.000000,G=0.000000,B=0.000000,A=1.000000)" "(R=0.000000,G=1.000000,B=0.000000,A=1.000000)" 0.5))
  (return (or _returnvalue_8 _returnvalue_7)))

(fn GetRunSpeed
  (return (Math|Float|Absolute(Float) (.y (Pawn|Components|CharacterMovement|GetLastUpdateVelocity (Variables|Character|GetCharacterMovement))))))