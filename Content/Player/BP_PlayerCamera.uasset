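; Player camera actor that becomes the view target and, after game start, eases toward the BP_CameraAnchor nearest the player.
; Each tick it interpolates orthographic width toward a target, keeping a SceneCapture2D in sync.
; Its position relative to anchor Y/Z bounds feeds an Offset parameter on the BP_PaintPostProcess painting material.
; An optional fill draws a time-scaled M_PaintingCircle into the RT_Mask render target.
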(event `self.ReceiveBeginPlay`
  (`self.SetCameraAnchors`)
  (`PlayerController.SetViewTargetWithBlend` (`GameplayStatics.GetPlayerController` 0) self 0.0 "VTBlend_Linear" 0.0 false)
  (bind _returnvalue (`GameplayStatics.GetActorOfClass` "/Game/Global/BP_PaintPostProcess.BP_PaintPostProcess_C"))
  (set `self.PaintPostProcess` _returnvalue)
  (`self.GetAnchorBounds`)
  (bind _asbp_game_mode (cast `/Game/BP_GameMode` (`GameplayStatics.GetGameMode`)))
  (add `/Game/BP_GameMode.GameStart` _asbp_game_mode (delegate `OnGameStart`))
  (bind _returnvalue_2 (`GameplayStatics.GetActorOfClass` "/Script/Engine.SceneCapture2D"))
  (set `self.SceneCapture` _returnvalue_2)
  (set `self.TargetSize` (`CameraComponent.OrthoWidth` (`self.CameraComponent`))))

(event `OnGameStart`
  (set `self.TargetSize` 6600.0)
  (set `self.DoTargetAnchor` true))

(event `self.ReceiveTick`
  (params (DeltaSeconds :type "Float (single-precision)"))
  (bind _cameracomponent (`self.CameraComponent`))
  (`|ExecutionSequence`
    (:`then_0`
      (`self.CalculateNDCOffset`)
      (if (`self.DoTargetAnchor`)
        (`self.LerpToClosestAnchor` DeltaSeconds)))
    (:`then_1`
      (bind _output_get (set `SceneCaptureComponent2D.OrthoWidth` (`KismetMathLibrary.FInterpTo` (`CameraComponent.OrthoWidth` _cameracomponent) (`self.TargetSize`) DeltaSeconds 3.0) (`SceneCapture2D.CaptureComponent2D` (`self.SceneCapture`))))
      (set `CameraComponent.OrthoWidth` _output_get _cameracomponent))
    (:`then_2`
      (`self.FillTexture`))))

(fn `CalculateNDCOffset`
  (locals (NewY :type "Float (double-precision)") (NewZ :type "Float (double-precision)"))
  (set `local.NewZ` (/ (- (.z (`self.K2_GetActorLocation`)) (`self.CameraMinZ`)) (`self.CameraMaxZ`) 2.0))
  (set `local.NewY` (/ (- (.y (`self.K2_GetActorLocation`)) (`self.CameraMinY`)) (`self.CameraMaxY`) 2.0))
  (bind _output_get (set `self.NDCOffset` (`KismetMathLibrary.MakeVector2D` (`local.NewY`) (`local.NewZ`))))
  (bind (_x _y) (`KismetMathLibrary.BreakVector2D` _output_get))
  (`MaterialInstanceDynamic.SetVectorParameterValue` (`/Game/Global/BP_PaintPostProcess.PaintingMatInstance` (`self.PaintPostProcess`)) "Offset" (`KismetMathLibrary.MakeColor` _x (- 1.0 _y))))

(fn `FillTexture`
  (if (`self.DoFill`)
    (bind (_canvas _size _context) (`KismetRenderingLibrary.BeginDrawCanvasToRenderTarget` "/Game/Global/Materials/Test/RT_Mask.RT_Mask"))
    (bind _returnvalue (`KismetMathLibrary.Lerp` 0.0 (`KismetMathLibrary.BreakVector2D` _size) (`self.FillTime`)))
    (`Canvas.K2_DrawMaterial` _canvas "/Game/Global/Materials/Test/M_PaintingCircle.M_PaintingCircle" (0.0 0.0) (`KismetMathLibrary.MakeVector2D` _returnvalue _returnvalue) (0.0 0.0) (1.0 1.0) 0.0 (0.5 0.5))
    (`KismetRenderingLibrary.EndDrawCanvasToRenderTarget` _context)
    (set `self.FillTime` (+ (`GameplayStatics.GetWorldDeltaSeconds`) (`self.FillTime`)))))

(fn `GetAnchorBounds`
  (for _array_element (`self.CameraAnchors`)
    (`|ExecutionSequence`
      (:`then_0`
        (bind (_returnvalue_x _returnvalue_y _returnvalue_z) (`KismetMathLibrary.BreakVector` (`self.K2_GetActorLocation` _array_element)))
        (if (< _returnvalue_y (`self.CameraMinY`))
          (set `self.CameraMinY` _returnvalue_y)))
      (:`then_1`
        (if (> _returnvalue_y (`self.CameraMaxY`))
          (set `self.CameraMaxY` _returnvalue_y)))
      (:`then_2`
        (if (< _returnvalue_z (`self.CameraMinZ`))
          (set `self.CameraMinZ` _returnvalue_z)))
      (:`then_3`
        (if (> _returnvalue_z (`self.CameraMaxZ`))
          (set `self.CameraMaxZ` _returnvalue_z))))))

(fn `GetClosestAnchor`
  (params (Pos :type "Vector Structure"))
  (returns (Anchor :type "/Game/Player/BP_CameraAnchor Object Reference"))
  (locals (ClosestAnchor :type "/Game/Player/BP_CameraAnchor Object Reference") (ClosestDistance :type "Float (double-precision)" :default 999999999.0))
  (for _array_element (`self.CameraAnchors`)
    (bind _returnvalue (`KismetMathLibrary.Vector_DistanceSquared` Pos (`self.K2_GetActorLocation` _array_element)))
    (if (< _returnvalue (`local.ClosestDistance`))
      (set `local.ClosestAnchor` _array_element)
      (set `local.ClosestDistance` _returnvalue)))
  (return (`local.ClosestAnchor`)))

(fn `LerpToClosestAnchor`
  (params (Delta :type "Float (single-precision)"))
  (bind _anchor (`self.GetClosestAnchor` (`self.K2_GetActorLocation` (`GameplayStatics.GetPlayerPawn` 0))))
  (bind _returnvalue (`self.K2_GetActorLocation` _anchor))
  (`self.K2_SetActorLocation` (`KismetMathLibrary.VInterpTo` (`self.K2_GetActorLocation`) (`KismetMathLibrary.SelectVector` _returnvalue (`KismetMathLibrary.MakeVector` (.x _returnvalue)) (not (`self.DoCenter`))) Delta (`self.CameraZorpSpeed`))))

(fn `ManageMaterialOffset`)

(fn `SetCameraAnchors`
  (bind _outactors (`GameplayStatics.GetAllActorsOfClass` "/Game/Player/BP_CameraAnchor.BP_CameraAnchor_C"))
  (set `self.CameraAnchors` _outactors))

(fn `UserConstructionScript`)