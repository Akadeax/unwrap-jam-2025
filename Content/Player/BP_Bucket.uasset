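; BP_Bucket is the level's finish trigger, which also paints at its own location two seconds after the game mode signals game start.
; When the player overlaps its Box, it hides the player mesh, spawns a BP_Endscreen_PC stand-in and clears input mappings.
; It then runs a delay-timed finale through BP_PlayerCamera, centering, widening the target size and triggering a fill, before showing WBP_FinScreen.
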(event `self.ReceiveBeginPlay`
  (bind _asbp_game_mode (cast `/Game/BP_GameMode` (`GameplayStatics.GetGameMode`)))
  (add `/Game/BP_GameMode.GameStart` _asbp_game_mode (delegate `CustomEvent`)))

(event `CustomEvent`
  (`KismetSystemLibrary.Delay` 2.0)
  (`/Game/Player/BP_PainterComponent.DoDraw` (`self.BP_PainterComponent`) (`self.K2_GetActorLocation`)))

(event `self.Box.OnComponentBeginOverlap`
  (params (OverlappedComponent :type "PrimitiveComponent Object Reference") (OtherActor :type "Actor Object Reference") (OtherComp :type "PrimitiveComponent Object Reference") (OtherBodyIndex :type Integer) (bFromSweep :type Boolean) (SweepResult :type "HitResult Structure (by ref)"))
  (bind _asbp_player_character (cast `/Game/Player/BP_PlayerCharacter` OtherActor))
  ; ChangePlayerMeshToDummyMesh
  (`SceneComponent.SetVisibility` (`Character.Mesh` _asbp_player_character) false true)
  (`|SpawnActorFromClass` "/Game/Player/BP_Endscreen_PC.BP_Endscreen_PC_C" (`KismetMathLibrary.MakeTransform` (+ (`self.FakePlayerPosition`) (`SceneComponent.K2_GetComponentLocation` (`self.DefaultSceneRoot`)))) "Undefined" "MultiplyWithRoot" null null)
  (`EnhancedInputSubsystemInterface.ClearAllMappings` (pcsubsystem `EnhancedInputLocalPlayerSubsystem` (`GameplayStatics.GetPlayerController` 0)))
  ; Comment
  (bind _returnvalue (`GameplayStatics.GetActorOfClass` "/Game/Player/BP_PlayerCamera.BP_PlayerCamera_C"))
  (set `/Game/Player/BP_PlayerCamera.DoCenter` true _returnvalue)
  (`KismetSystemLibrary.Delay` (`self.CameraDelay`))
  (set `/Game/Player/BP_PlayerCamera.TargetSize` 13200.0 _returnvalue)
  (`KismetSystemLibrary.Delay` (`self.ColorDelay`))
  (set `/Game/Player/BP_PlayerCamera.DoFill` true _returnvalue)
  (`KismetSystemLibrary.Delay` (`self.EndScreenDelay`))
  (bind _returnvalue_2 (`|GenericCreateObject` "/Game/Player/WBP_FinScreen.WBP_FinScreen_C"))
  (`UserWidget.AddToViewport` _returnvalue_2 0))

(fn `UserConstructionScript`)