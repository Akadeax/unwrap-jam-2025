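; Tutorial trigger volume that shows a tutorial widget the first time the player character overlaps its Box.
; The overlap reveals and initializes the Widget, sets IsActive and HasPlayed so it fires only once, and prints a leftover debug string.
; While active, Tick polls the widget's Check to update IsActive; when inactive, it sets the widget hidden every frame.
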(event `self.ReceiveTick`
  (params (DeltaSeconds :type "Float (single-precision)"))
  (bind _widget (`self.widget`))
  (if (`self.IsActive`)
    (bind _result (`/Game/Player/tut/BP_BaseTut.Check` _widget))
    (set `self.IsActive` _result)
    (else
      (`/Game/Player/tut/BP_BaseTut.SetVisibility` _widget (`self.IsActive`)))))

(event `self.Box.OnComponentBeginOverlap`
  (params (OverlappedComponent :type "PrimitiveComponent Object Reference") (OtherActor :type "Actor Object Reference") (OtherComp :type "PrimitiveComponent Object Reference") (OtherBodyIndex :type Integer) (bFromSweep :type Boolean) (SweepResult :type "HitResult Structure (by ref)"))
  (bind _widget (`self.widget`))
  (if (not (`self.HasPlayed`))
    (cast `/Game/Player/BP_PlayerCharacter` OtherActor)
    (`/Game/Player/tut/BP_BaseTut.SetVisibility` _widget true)
    (set `self.IsActive` true)
    (`/Game/Player/tut/BP_BaseTut.Init` _widget)
    (set `self.HasPlayed` true)
    (`KismetSystemLibrary.PrintString` "AAAAAAAAAAAAAAAA")))

(fn `UserConstructionScript`)