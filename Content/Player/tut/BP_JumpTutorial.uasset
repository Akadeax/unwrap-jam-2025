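; Jump tutorial Blueprint that detects whether the player has jumped.
; On BeginPlay it binds to the OnJump dispatcher of player 0's BP_PlayerCharacter and sets a Jumped flag when it fires.
; Check returns that flag, and SetVisibility shows or hides its Widget.
; The flag is never reset within this Blueprint.
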(event `self.ReceiveBeginPlay`
  (`parent.ReceiveBeginPlay`)
  (bind _asbp_player_character (cast `/Game/Player/BP_PlayerCharacter` (`GameplayStatics.GetPlayerPawn` 0)))
  (add `/Game/Player/BP_PlayerCharacter.OnJump` _asbp_player_character (delegate `CustomEvent`)))

(event `CustomEvent`
  (set `self.jumped` true))

(fn `Check`
  (returns (Result :type Boolean))
  (return (`self.jumped`)))

(fn `SetVisibility`
  (params (visibility :type Boolean))
  (`SceneComponent.SetVisibility` (`self.Widget`) visibility false))

(fn `UserConstructionScript`
  (`parent.UserConstructionScript`))