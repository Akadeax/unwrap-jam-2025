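; BP_DashTutorial is a tutorial step that tracks whether the player has performed a dash.
; Init casts the player pawn to BP_PlayerCharacter and binds to its OnDash event; an auto-generated handler function sets the Dashed flag.
; Check returns that flag, and SetVisibility shows or hides the tutorial widget.
; BeginPlay and construction only call the parent.
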(event `self.ReceiveBeginPlay`
  (`parent.ReceiveBeginPlay`))

(fn `BP_DashTutorial_AutoGenFunc`
  (set `self.Dashed` true))

(fn `Check`
  (returns (Result :type Boolean))
  (return (`self.Dashed`)))

(fn `Init`
  (bind _asbp_player_character (cast `/Game/Player/BP_PlayerCharacter` (`GameplayStatics.GetPlayerPawn` 0)))
  (add `/Game/Player/BP_PlayerCharacter.OnDash` _asbp_player_character (`|CreateDelegate` :!event `BP_DashTutorial_AutoGenFunc`)))

(fn `SetVisibility`
  (params (visibility :type Boolean))
  (`SceneComponent.SetVisibility` (`self.Widget`) visibility false))

(fn `UserConstructionScript`
  (`parent.UserConstructionScript`))