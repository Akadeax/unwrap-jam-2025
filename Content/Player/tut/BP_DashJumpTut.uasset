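; Tutorial step that teaches the dash-jump, completed when the player jumps shortly after dashing.
; Init binds handlers to the player character's jump and dash events, and Tick times the gap after a dash.
; The jump handler stops the timer and sets Finished if it is under a short threshold, without testing whether a dash is active.
; Check returns true until finished, and SetVisibility toggles the prompt widget.
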(event `self.ReceiveBeginPlay`
  (`parent.ReceiveBeginPlay`))

(event `self.ReceiveTick`
  (params (DeltaSeconds :type "Float (single-precision)"))
  (if (`self.Dashed`)
    (set `self.TimeSinceDash` (+ DeltaSeconds (`self.TimeSinceDash`)))))

(fn `BP_DashJumpTut_AutoGenFunc`
  (set `self.Dashed` true)
  (set `self.TimeSinceDash` 0.0))

(fn `BP_DashJumpTut_AutoGenFunc1`
  (set `self.Dashed` false)
  (if (< (`self.TimeSinceDash`) 0.65)
    (set `self.Finished` true)))

(fn `Check`
  (returns (Result :type Boolean))
  (return (not (`self.Finished`))))

(fn `Init`
  (bind _asbp_player_character (cast `/Game/Player/BP_PlayerCharacter` (`GameplayStatics.GetPlayerPawn` 0)))
  (add `/Game/Player/BP_PlayerCharacter.OnJump` _asbp_player_character (`|CreateDelegate` :!event `BP_DashJumpTut_AutoGenFunc1`))
  (add `/Game/Player/BP_PlayerCharacter.OnDash` _asbp_player_character (`|CreateDelegate` :!event `BP_DashJumpTut_AutoGenFunc`)))

(fn `SetVisibility`
  (params (visibility :type Boolean))
  (`SceneComponent.SetVisibility` (`self.Widget`) visibility false))

(fn `UserConstructionScript`
  (`parent.UserConstructionScript`))