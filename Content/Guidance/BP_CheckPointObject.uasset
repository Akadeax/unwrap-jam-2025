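; BP_CheckPointObject is a guidance checkpoint that moves a BP_FollowObject along an ordered route as the player advances.
; On BeginPlay it caches the level's follow object and links to the checkpoint whose Index is one higher than its own.
; When the player character overlaps its box, it passes that next checkpoint to the follow object, or destroys the follow object if none exists.
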(event `self.ReceiveBeginPlay`
  (`|ExecutionSequence`
    (:`then_0`
      (bind _returnvalue (`GameplayStatics.GetActorOfClass` "/Game/Guidance/BP_FollowObject.BP_FollowObject_C"))
      (if (`KismetSystemLibrary.IsValid` _returnvalue)
        (set `self.FollowObject` _returnvalue)))
    (:`then_1`
      (bind _outactors (`GameplayStatics.GetAllActorsOfClass` "BP_CheckPointObject_C"))
      (for _array_element _outactors
        (if (== (`/Game/Guidance/BP_CheckPointObject.index` _array_element) (+ (`self.index`) 1))
          (set `self.NextCheckPoint` _array_element))))))

(event `self.Box.OnComponentBeginOverlap`
  (params (OverlappedComponent :type "PrimitiveComponent Object Reference") (OtherActor :type "Actor Object Reference") (OtherComp :type "PrimitiveComponent Object Reference") (OtherBodyIndex :type Integer) (bFromSweep :type Boolean) (SweepResult :type "HitResult Structure (by ref)"))
  (bind _followobject (`self.FollowObject`))
  (bind _nextcheckpoint (`self.NextCheckPoint`))
  (cast `/Game/Player/BP_PlayerCharacter` OtherActor)
  (if (`KismetSystemLibrary.IsValid` _nextcheckpoint)
    (`/Game/Guidance/BP_FollowObject.SetNewCheckPoint` _followobject _nextcheckpoint)
    (else
      (`self.K2_DestroyActor` _followobject))))

(fn `UserConstructionScript`)