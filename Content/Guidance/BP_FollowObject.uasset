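; BP_FollowObject is a guide actor that glides to the current goal checkpoint and controls which platform particle effects are visible.
; On BeginPlay it caches all BP_PlatformParticles and applies its initial GoalCheckPoint.
; SetNewCheckPoint stores the goal and shows only particles whose Index is within one of the checkpoint's.
; Tick eases the actor toward the goal with VInterpTo; its distance check has no effect.
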(event `self.ReceiveBeginPlay`
  (bind _outactors (`GameplayStatics.GetAllActorsOfClass` "/Game/Global/BP_PlatformParticles.BP_PlatformParticles_C"))
  (set `self.Sparkles` _outactors)
  (`self.SetNewCheckPoint` (`self.GoalCheckPoint`)))

(event `self.ReceiveTick`
  (params (DeltaSeconds :type "Float (single-precision)"))
  (bind _goalcheckpoint (`self.GoalCheckPoint`))
  (if (`KismetSystemLibrary.IsValid` _goalcheckpoint)
    (if (> (`KismetMathLibrary.Vector_DistanceSquared` (`self.K2_GetActorLocation`) (`self.K2_GetActorLocation` _goalcheckpoint)) 10.0)
      _
      (else
        _))
    (`self.K2_SetActorLocation` (`KismetMathLibrary.VInterpTo` (`self.K2_GetActorLocation`) (`self.K2_GetActorLocation` (`self.GoalCheckPoint`)) DeltaSeconds 5.0))))

(fn `SetNewCheckPoint`
  (params (CheckPoint :type "/Game/Guidance/BP_CheckPointObject Object Reference"))
  (bind _output_get (set `self.GoalCheckPoint` CheckPoint))
  (for _array_element (`self.Sparkles`)
    (bind _index (`/Game/Guidance/BP_CheckPointObject.index` _output_get))
    (bind _index_2 (`/Game/Global/BP_PlatformParticles.Index` _array_element))
    (`SceneComponent.SetVisibility` (`/Game/Global/BP_PlatformParticles.DefaultSceneRoot` _array_element) (and (<= _index (+ _index_2 1)) (>= _index (- _index_2 1))) true)))

(fn `UserConstructionScript`)